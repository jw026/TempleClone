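; BP_RoadTileUpSlope is an up-slope road tile that hands off to a road master actor as the player passes, then removes itself.
; When the player character overlaps its box collider, it finds BP_RoadMaster and calls TestMessage with the NextAttachPoint world location as the next spawn point, plus itself.
; It then destroys itself after a short delay.
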(event OnComponentBeginOverlap(BoxCollider)
  (params (OverlappedComponent :type Primitive%20Component%20Object%20Reference) (OtherActor :type Actor%20Object%20Reference) (OtherComp :type Primitive%20Component%20Object%20Reference) (OtherBodyIndex :type Integer) (bFromSweep :type Boolean) (SweepResult :type Hit%20Result%20Structure%20%28by%20ref%29))
  (if (== OtherActor (Game|GetPlayerCharacter 0))
    (bind _returnvalue (Actor|GetActorOfClass "/Game/Blueprints/BP_RoadMAster.BP_RoadMaster_C"))
    (Class|BPIEndlessRoad|Test(Message) _returnvalue (Transformation|GetWorldLocation (Variables|Default|GetNextAttachPoint)) self)
    (Utilities|FlowControl|Delay 0.5)
    (Actor|DestroyActor)))

(event EventBeginPlay)

(event Collision|EventActorBeginOverlap
  (params (OtherActor :type Actor%20Object%20Reference)))

(event EventTick
  (params (DeltaSeconds :type Float%20%28single-precision%29)))

(fn ConstructionScript
  (|CallParentFunction))