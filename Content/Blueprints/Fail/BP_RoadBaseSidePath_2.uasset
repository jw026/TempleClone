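; Road tile variant that places its path at random to one side or in the center, apparently for an endless runner.
; The construction script picks the road's Y offset, showing one railing for side positions and none for center.
; The first trigger overlap calls SpawnNew, then destroys the tile after a short delay, while the kill box calls EndGame on the player.
; SpawnObstacle is overridden empty, skipping the parent's obstacle spawning.
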(event OnComponentBeginOverlap(TriggerBox)
  (params (OverlappedComponent :type Primitive%20Component%20Object%20Reference) (OtherActor :type Actor%20Object%20Reference) (OtherComp :type Primitive%20Component%20Object%20Reference) (OtherBodyIndex :type Integer) (bFromSweep :type Boolean) (SweepResult :type Hit%20Result%20Structure%20%28by%20ref%29))
  (Utilities|FlowControl|DoOnce false
    (:Completed
      (CallFunction|SpawnNew OtherActor)
      (Utilities|FlowControl|Delay 2.0)
      (Actor|DestroyActor))))

(event OnComponentBeginOverlap(KillBox)
  (params (OverlappedComponent :type Primitive%20Component%20Object%20Reference) (OtherActor :type Actor%20Object%20Reference) (OtherComp :type Primitive%20Component%20Object%20Reference) (OtherBodyIndex :type Integer) (bFromSweep :type Boolean) (SweepResult :type Hit%20Result%20Structure%20%28by%20ref%29))
  (bind _asbp_player (Utilities|Casting|CastToBP_Player OtherActor))
  (Default|EndGame _asbp_player))

(event EventBeginPlay
  (|CallParentFunction) ; This node is disabled and will not be called.\nDrag off pins to build functionality.
)

(event Collision|EventActorBeginOverlap
  (params (OtherActor :type Actor%20Object%20Reference))
  (|CallParentFunction OtherActor) ; This node is disabled and will not be called.\nDrag off pins to build functionality.
)

(event EventTick
  (params (DeltaSeconds :type Float%20%28single-precision%29))
  (|CallParentFunction DeltaSeconds) ; This node is disabled and will not be called.\nDrag off pins to build functionality.
)

(fn ConstructionScript
  (bind _roadroot (Variables|Default|GetRoadRoot))
  (bind _l_railing (Variables|Default|GetL_Railing))
  (bind _r_railing (Variables|Default|GetR_Railing))
  (switch int (Math|Random|RandomIntegerinRange 0 2)
    (:Default
      (Transformation|SetRelativeLocation _roadroot (Math|Vector|MakeVector 0.0 0.0 15.0) false false :!label _label)
      (Rendering|SetVisibility _l_railing false false)
      (Rendering|SetVisibility _r_railing false false))
    (:0
      (Transformation|SetRelativeLocation _roadroot (Math|Vector|MakeVector 0.0 -3.3e+02 15.0) false false)
      (Rendering|SetVisibility _l_railing true false)
      (Rendering|SetVisibility _r_railing false false))
    (:1
      (goto _label))
    (:2
      (Transformation|SetRelativeLocation _roadroot (Math|Vector|MakeVector 0.0 3.3e+02 15.0) false false)
      (Rendering|SetVisibility (Variables|Default|GetL_Railing) false false)
      (Rendering|SetVisibility (Variables|Default|GetR_Railing) true false)))
  (|CallParentFunction))

(fn SpawnObstacle)