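; Game mode that builds a chain of randomly chosen road tiles when play begins.
; BeginPlay calls AddNewTile ten times, each spawning a class picked from TypeOfTile at NextSpawnPoint.
; Each tile cast to BP_RoadTileBase supplies its NextAttachPoint location as the next spawn point, with zero rotation and unit scale.
; The inclusive random range runs up to the array length, so it can pick an index past the end.
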(event EventBeginPlay
  (for _index (range 0 9)
    (CallFunction|AddNewTile)))

(event EventTick
  (params (DeltaSeconds :type Float%20%28single-precision%29)))

(fn ConstructionScript)

(fn AddNewTile
  (bind _typeoftile (Variables|Default|GetTypeOfTile))
  (bind _returnvalue (Game|SpawnActorfromClass (Utilities|Array|Get(acopy) _typeoftile (Math|Random|RandomIntegerinRange 0 (Utilities|Array|Length _typeoftile))) (Variables|Default|GetNextSpawnPoint) "Undefined" 0 0))
  (bind _asbp_road_tile_base (Utilities|Casting|CastToBP_RoadTileBase _returnvalue))
  (Variables|Default|SetNextSpawnPoint (Math|Transform|MakeTransform (Transformation|GetWorldLocation (Variables|/Game/Blueprints/BP_RoadTileBase.BP_RoadTileBase_C|GetNextAttachPoint _asbp_road_tile_base)) "0, 0, 0" "1,1,1")))