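; BP_Player_PawnTest is a player pawn that moves forward continuously and steps sideways between lanes, in the style of a lane runner.
; Tick offsets it by its forward vector scaled by ForwardSpeed and delta time, without sweeping for collision.
; MoveRight and MoveLeft presses shift it by MoveLength along world Y, with a Position counter whose bounds limit how far it can step each way.
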(event EventTick
  (params (DeltaSeconds :type Float%20%28single-precision%29))
  ;[1 1 1] Move Forward
  (Transformation|AddActorLocalOffset (* (* (Transformation|GetActorForwardVector) (Variables|Default|GetForward%20Speed)) DeltaSeconds) false false))

(event Input|ActionEvents|InputActionMoveRight
  (params (Key :type Key%20Structure :default "None"))
  ;[1 1 1] Move Left / Right
  (:Pressed
    (if (<= (Variables|Default|GetPosition) 1)
      (Math|Integer|IncrementInt (Variables|Default|GetPosition)
        (:%20%20
          (Transformation|AddActorWorldOffset (Math|Vector|MakeVector 0.0 (Variables|Default|GetMove%20Length) 0.0)))))))

(event Input|ActionEvents|InputActionMoveLeft
  (params (Key :type Key%20Structure :default "None"))
  ;[1 1 1] Move Left / Right
  (:Pressed
    (if (>= (Variables|Default|GetPosition) 1)
      (Math|Integer|DecrementInt (Variables|Default|GetPosition)
        (:%20%20
          (Transformation|AddActorWorldOffset (Math|Vector|MakeVector 0.0 (* (Variables|Default|GetMove%20Length) -1.0) 0.0)))))))

(event Input|ActionEvents|InputActionJump
  (params (Key :type Key%20Structure :default "None")))

(fn ConstructionScript)