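; BP_RoadBase_Type_01 is a road segment that asks BP_RoadMaster to continue the road as the player advances.
; Its TriggerBox fires once, calls TestMessage on the master if the player overlapped, then destroys the segment after a delay, whatever triggered it.
; GetNextTransform exposes the NextSpawnPoint transform for chaining segments.
; Random obstacle spawning via child actor components and segment movement exist but are never run.
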(event OnComponentBeginOverlap(TriggerBox)
  (params (OverlappedComponent :type Primitive%20Component%20Object%20Reference) (OtherActor :type Actor%20Object%20Reference) (OtherComp :type Primitive%20Component%20Object%20Reference) (OtherBodyIndex :type Integer) (bFromSweep :type Boolean) (SweepResult :type Hit%20Result%20Structure%20%28by%20ref%29))
  (Utilities|FlowControl|DoOnce false
    (:Completed
      (CallFunction|SpawnNew OtherActor)
      (Utilities|FlowControl|Delay 2.0)
      (Actor|DestroyActor))))

(event EventBeginPlay
  (bind _returnvalue (Actor|GetActorOfClass "/Game/Blueprints/BP_RoadMAster.BP_RoadMaster_C"))
  (Variables|Default|SetRoadMaster_Ref _returnvalue))

(event Collision|EventActorBeginOverlap
  (params (OtherActor :type Actor%20Object%20Reference)))

(event EventTick
  (params (DeltaSeconds :type Float%20%28single-precision%29)))

(fn ConstructionScript)

(fn SpawnNew
  (params (NewParam :type Actor%20Object%20Reference))
  (if (== NewParam (Game|GetPlayerCharacter 0))
    (Class|BPIEndlessRoad|Test(Message) (Variables|Default|GetRoadMaster_Ref) "0, 0, 0")
    (return)
    (else
      (Development|PrintString "Fail on overlap"))))

(fn GetNextTransform
  (return (Transformation|GetWorldTransform (Variables|Default|GetNextSpawnPoint)) ""))

(fn GetSpawnTransform)

(fn SpawnObstacle
  (bind _returnvalue (Math|Random|RandomIntegerinRange 0 2))
  (bind _spawnpointarray (Variables|Default|GetSpawnPointArray))
  (bind _returnvalue_2 (Utilities|Array|LastIndex _spawnpointarray))
  (bind _returnvalue_3 (Math|Random|RandomIntegerinRange 0 _returnvalue_2))
  (bind _output (Utilities|Array|Get(acopy) _spawnpointarray _returnvalue_3))
  (if (== _returnvalue_3 2)
    (switch int _returnvalue
      (:Default
        (switch int _returnvalue :!label _label
          (:Default
            (AddComponent|AddChildActorComponent false _output :!label _label_2))
          (:0
            (AddComponent|AddChildActorComponent false _output :!label _label_3))
          (:1
            (goto _label_3))
          (:2
            (goto _label_2))))
      (:0
        (goto _label))
      (:1
        (AddComponent|AddChildActorComponent false (Utilities|Array|Get(acopy) _spawnpointarray 2)))
      (:2
        (goto _label)))
    (else
      (goto _label))))