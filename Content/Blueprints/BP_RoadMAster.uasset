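; Endless road manager that creates the score HUD, lays ten random base tiles at BeginPlay and tracks score.
; Each Test event adds score and spawns one tile at the transform returned by the previous tile's GetNextTransform.
; Randomized count marks insert slope, side-path and jump tiles among five base variants; jumps reset the count and raise player speed.
; Crossroad branching and an older spawn chain remain in the graph but never run.
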(event Custom|AddPoints
  (params (AddScore :type Integer)))

(event EventBeginPlay
  ;[1 1 1] At start of game, create and add widget then spawn 10 normal tiles
  (Utilities|FlowControl|Sequence
    (:then_0
      (bind _returnvalue (UserInterface|CreateWidget "/Game/Widgets/PlayerHUD.PlayerHUD_C" (Game|GetPlayerController 0)))
      (Variables|Default|SetPlayerWidget _returnvalue)
      (UserInterface|Viewport|AddtoViewport (Variables|Default|GetPlayerWidget) 0)
      (bind _asbp_player (Utilities|Casting|CastToBP_Player (Game|GetPlayerCharacter 0)))
      (Variables|Default|SetPlayer_Ref _asbp_player))
    (:then_1
      (Variables|Default|SetSlopeTile (Math|Random|RandomIntegerinRange 15 30))
      (Variables|Default|SetSideTile (Math|Random|RandomIntegerinRange 5 15)))
    (:then_2
      (for _index (range 0 9)
        (switch int (Math|Random|RandomIntegerinRange 0 4)
          (:Default
            ;[1 1 1] When called, spawn a new base tile at end of road
            (Math|Integer|IncrementInt (Variables|Default|GetTileCount) :!label _label
              (:%20%20
                (bind _returnvalue_2 (Game|SpawnActorfromClass "/Game/Blueprints/BP_RoadBase_Type_02.BP_RoadBase_Type_02_C" (Variables|Default|GetNextSpawnTrans) "Undefined" 0 0))
                (bind _nextpoint (Default|GetNextTransform _returnvalue_2))
                (Variables|Default|SetNextSpawnTrans _nextpoint)
                (Development|PrintString (Utilities|String|ToString(Integer) (Variables|Default|GetTileCount)))
                (Development|PrintString (Utilities|String|Append "Tiles passed = " (Utilities|String|ToString(Integer) (Variables|Default|GetTilesPassed)))))))
          (:0
            (goto _label))
          (:1
            (Math|Integer|IncrementInt (Variables|Default|GetTileCount)
              (:%20%20
                (bind _returnvalue_3 (Game|SpawnActorfromClass "/Game/Blueprints/BP_RoadBase_Type_03.BP_RoadBase_Type_03_C" (Variables|Default|GetNextSpawnTrans) "Undefined" 0 0))
                (bind _nextpoint_2 (Default|GetNextTransform _returnvalue_3))
                (Variables|Default|SetNextSpawnTrans _nextpoint_2)
                (Development|PrintString (Utilities|String|ToString(Integer) (Variables|Default|GetTileCount)))
                (Development|PrintString (Utilities|String|Append "Tiles passed = " (Utilities|String|ToString(Integer) (Variables|Default|GetTilesPassed)))))))
          (:2
            (Math|Integer|IncrementInt (Variables|Default|GetTileCount)
              (:%20%20
                (bind _returnvalue_4 (Game|SpawnActorfromClass "/Game/Blueprints/BP_RoadBase_Type_04.BP_RoadBase_Type_04_C" (Variables|Default|GetNextSpawnTrans) "Undefined" 0 0))
                (bind _nextpoint_3 (Default|GetNextTransform _returnvalue_4))
                (Variables|Default|SetNextSpawnTrans _nextpoint_3)
                (Development|PrintString (Utilities|String|ToString(Integer) (Variables|Default|GetTileCount)))
                (Development|PrintString (Utilities|String|Append "Tiles passed = " (Utilities|String|ToString(Integer) (Variables|Default|GetTilesPassed)))))))
          (:3
            (Math|Integer|IncrementInt (Variables|Default|GetTileCount)
              (:%20%20
                (bind _returnvalue_5 (Game|SpawnActorfromClass "/Game/Blueprints/BP_RoadBase_Type_06.BP_RoadBase_Type_06_C" (Variables|Default|GetNextSpawnTrans) "Undefined" 0 0))
                (bind _nextpoint_4 (Default|GetNextTransform _returnvalue_5))
                (Variables|Default|SetNextSpawnTrans _nextpoint_4)
                (Development|PrintString (Utilities|String|ToString(Integer) (Variables|Default|GetTileCount)))
                (Development|PrintString (Utilities|String|Append "Tiles passed = " (Utilities|String|ToString(Integer) (Variables|Default|GetTilesPassed)))))))
          (:4
            (Math|Integer|IncrementInt (Variables|Default|GetTileCount)
              (:%20%20
                (bind _returnvalue_6 (Game|SpawnActorfromClass "/Game/Blueprints/BP_RoadBase_Type_05.BP_RoadBase_Type_05_C" (Variables|Default|GetNextSpawnTrans) "Undefined" 0 0))
                (bind _nextpoint_5 (Default|GetNextTransform _returnvalue_6))
                (Variables|Default|SetNextSpawnTrans _nextpoint_5)
                (Development|PrintString (Utilities|String|ToString(Integer) (Variables|Default|GetTileCount)))
                (Development|PrintString (Utilities|String|Append "Tiles passed = " (Utilities|String|ToString(Integer) (Variables|Default|GetTilesPassed))))))))))))

(event EventAddPointsInterface
  (params (Points :type Integer))
  (Variables|Default|SetCurrentScore (+ Points (Variables|Default|GetCurrentScore)))
  (Default|UpdateScore (Variables|Default|GetPlayerWidget) (Variables|Default|GetCurrentScore))
  (Development|PrintString (Utilities|String|ToString(Integer) (Variables|Default|GetCurrentScore))))

(event EventTest
  (params (NextSpawnPoint :type Vector :default "0, 0, 0") (TargetActor :type Actor%20Object%20Reference))
  ;[1 1 1] Add / Update score
  (Math|Integer|IncrementInt (Variables|Default|GetTilesPassed)
    (:%20%20
      (CallFunction|AddPointsInterface (Variables|Default|GetScore))
      (Development|PrintString "Fire fire fire")
      ;[1 1 1] Set spawn mark for slopetile and check which tile to spawn
      (if (== (Variables|Default|GetTileCount) (Variables|Default|GetSlopeTile))
        ;[1 1 1] At reached mark, spawn a slope tile at end of road
        (Math|Integer|IncrementInt (Variables|Default|GetTileCount)
          (:%20%20
            (Variables|Default|SetNewSlopeTile (Math|Random|RandomIntegerinRange 15 30))
            (if (== (+ (Variables|Default|GetNewSlopeTile) 1) (Variables|Default|GetSlopeTile))
              (Variables|Default|SetSlopeTile (+ (Variables|Default|GetNewSlopeTile) 2))
              (else
                (Variables|Default|SetSlopeTile (Variables|Default|GetNewSlopeTile))))
            (bind _returnvalue (Game|SpawnActorfromClass "/Game/Blueprints/BP_RoadBaseUpSlope.BP_RoadBaseUpSlope_C" (Variables|Default|GetNextSpawnTrans) "Undefined" 0 0))
            (bind _nextpoint (Default|GetNextTransform _returnvalue))
            (Variables|Default|SetNextSpawnTrans _nextpoint)
            (Development|PrintString (Utilities|String|ToString(Integer) (Variables|Default|GetTileCount)))))
        (elif (== (Variables|Default|GetTileCount) (Variables|Default|GetSideTile))
          ;[1 1 1] At reached mark, spawn a side tile at end of road
          (Math|Integer|IncrementInt (Variables|Default|GetTileCount)
            (:%20%20
              (Variables|Default|SetNewSideTile (Math|Random|RandomIntegerinRange 5 15))
              (if (== (+ (Variables|Default|GetNewSideTile) 1) (Variables|Default|GetSideTile))
                (Variables|Default|SetSideTile (+ (Variables|Default|GetNewSideTile) 2))
                (else
                  (Variables|Default|SetSideTile (Variables|Default|GetNewSideTile))))
              (bind _returnvalue_2 (Game|SpawnActorfromClass "/Game/Blueprints/BP_RoadBaseSidePath.BP_RoadBaseSidePath_C" (Variables|Default|GetNextSpawnTrans) "Undefined" 0 0))
              (bind _nextpoint_2 (Default|GetNextTransform _returnvalue_2))
              (Variables|Default|SetNextSpawnTrans _nextpoint_2)
              (Development|PrintString (Utilities|String|ToString(Integer) (Variables|Default|GetTileCount)))))
          (elif (>= (Variables|Default|GetTileCount) (Variables|Default|GetTilesBeforeNextType))
            ;[1 1 1] At reached mark, reset tile count, make a new mark and spawn a jump tile at end of road
            (Variables|Default|SetTileCount 1)
            (Variables|Default|SetTilesBeforeNextType (Math|Random|RandomIntegerinRange 40 50))
            (bind _returnvalue_3 (Game|SpawnActorfromClass "/Game/Blueprints/BP_RoadJump.BP_RoadJump_C" (Variables|Default|GetNextSpawnTrans) "Undefined" 0 0))
            (bind _nextpoint_3 (Default|GetNextTransform _returnvalue_3))
            (Variables|Default|SetNextSpawnTrans _nextpoint_3)
            (Development|PrintString (Utilities|String|ToString(Integer) (Variables|Default|GetTileCount)))
            (Default|IncreaseMoveSpeed (Variables|Default|GetPlayer_Ref))
            (else
              (switch int (Math|Random|RandomIntegerinRange 0 4)
                (:Default
                  ;[1 1 1] When called, spawn a new base tile at end of road
                  (Math|Integer|IncrementInt (Variables|Default|GetTileCount) :!label _label
                    (:%20%20
                      (bind _returnvalue_4 (Game|SpawnActorfromClass "/Game/Blueprints/BP_RoadBase_Type_02.BP_RoadBase_Type_02_C" (Variables|Default|GetNextSpawnTrans) "Undefined" 0 0))
                      (bind _nextpoint_4 (Default|GetNextTransform _returnvalue_4))
                      (Variables|Default|SetNextSpawnTrans _nextpoint_4)
                      (Development|PrintString (Utilities|String|ToString(Integer) (Variables|Default|GetTileCount)))
                      (Development|PrintString (Utilities|String|Append "Tiles passed = " (Utilities|String|ToString(Integer) (Variables|Default|GetTilesPassed)))))))
                (:0
                  (goto _label))
                (:1
                  (Math|Integer|IncrementInt (Variables|Default|GetTileCount)
                    (:%20%20
                      (bind _returnvalue_5 (Game|SpawnActorfromClass "/Game/Blueprints/BP_RoadBase_Type_03.BP_RoadBase_Type_03_C" (Variables|Default|GetNextSpawnTrans) "Undefined" 0 0))
                      (bind _nextpoint_5 (Default|GetNextTransform _returnvalue_5))
                      (Variables|Default|SetNextSpawnTrans _nextpoint_5)
                      (Development|PrintString (Utilities|String|ToString(Integer) (Variables|Default|GetTileCount)))
                      (Development|PrintString (Utilities|String|Append "Tiles passed = " (Utilities|String|ToString(Integer) (Variables|Default|GetTilesPassed)))))))
                (:2
                  (Math|Integer|IncrementInt (Variables|Default|GetTileCount)
                    (:%20%20
                      (bind _returnvalue_6 (Game|SpawnActorfromClass "/Game/Blueprints/BP_RoadBase_Type_04.BP_RoadBase_Type_04_C" (Variables|Default|GetNextSpawnTrans) "Undefined" 0 0))
                      (bind _nextpoint_6 (Default|GetNextTransform _returnvalue_6))
                      (Variables|Default|SetNextSpawnTrans _nextpoint_6)
                      (Development|PrintString (Utilities|String|ToString(Integer) (Variables|Default|GetTileCount)))
                      (Development|PrintString (Utilities|String|Append "Tiles passed = " (Utilities|String|ToString(Integer) (Variables|Default|GetTilesPassed)))))))
                (:3
                  (Math|Integer|IncrementInt (Variables|Default|GetTileCount)
                    (:%20%20
                      (bind _returnvalue_7 (Game|SpawnActorfromClass "/Game/Blueprints/BP_RoadBase_Type_06.BP_RoadBase_Type_06_C" (Variables|Default|GetNextSpawnTrans) "Undefined" 0 0))
                      (bind _nextpoint_7 (Default|GetNextTransform _returnvalue_7))
                      (Variables|Default|SetNextSpawnTrans _nextpoint_7)
                      (Development|PrintString (Utilities|String|ToString(Integer) (Variables|Default|GetTileCount)))
                      (Development|PrintString (Utilities|String|Append "Tiles passed = " (Utilities|String|ToString(Integer) (Variables|Default|GetTilesPassed)))))))
                (:4
                  (Math|Integer|IncrementInt (Variables|Default|GetTileCount)
                    (:%20%20
                      (bind _returnvalue_8 (Game|SpawnActorfromClass "/Game/Blueprints/BP_RoadBase_Type_05.BP_RoadBase_Type_05_C" (Variables|Default|GetNextSpawnTrans) "Undefined" 0 0))
                      (bind _nextpoint_8 (Default|GetNextTransform _returnvalue_8))
                      (Variables|Default|SetNextSpawnTrans _nextpoint_8)
                      (Development|PrintString (Utilities|String|ToString(Integer) (Variables|Default|GetTileCount)))
                      (Development|PrintString (Utilities|String|Append "Tiles passed = " (Utilities|String|ToString(Integer) (Variables|Default|GetTilesPassed)))))))))))))))

(fn ConstructionScript)