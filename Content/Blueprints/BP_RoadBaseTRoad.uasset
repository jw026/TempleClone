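; T-junction road tile, child of a base road class, randomly picked as one of three crossroad types on construction.
; The type positions or hides a railing and decides whether GetNextTransform returns either or both next spawn points.
; Construction also caches world transforms for three left and three right lanes.
; SpawnObstacle is overridden empty, and the rotation trigger only casts to BP_Player with no further logic.
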(event OnComponentBeginOverlap(RotationTrigger)
  (params (OverlappedComponent :type Primitive%20Component%20Object%20Reference) (OtherActor :type Actor%20Object%20Reference) (OtherComp :type Primitive%20Component%20Object%20Reference) (OtherBodyIndex :type Integer) (bFromSweep :type Boolean) (SweepResult :type Hit%20Result%20Structure%20%28by%20ref%29))
  (Utilities|Casting|CastToBP_Player OtherActor))

(event EventBeginPlay
  (|CallParentFunction) ; This node is disabled and will not be called.\nDrag off pins to build functionality.
)

(event Collision|EventActorBeginOverlap
  (params (OtherActor :type Actor%20Object%20Reference))
  (|CallParentFunction OtherActor) ; This node is disabled and will not be called.\nDrag off pins to build functionality.
)

(event EventTick
  (params (DeltaSeconds :type Float%20%28single-precision%29))
  (|CallParentFunction DeltaSeconds) ; This node is disabled and will not be called.\nDrag off pins to build functionality.
)

(fn ConstructionScript
  (bind _r_railing (Variables|Default|GetR_Railing))
  (bind _r_railing_2 (Variables|Default|GetR_Railing))
  (switch int (Math|Random|RandomIntegerinRange 0 2)
    (:Default
      (Rendering|SetVisibility _r_railing false false :!label _label)
      (Variables|Default|SetTypeOfCrossroad 1))
    (:0
      (Transformation|SetRelativeLocation _r_railing_2 (Math|Vector|MakeVector 0.0 55.0 0.0) false false)
      (Rendering|SetVisibility _r_railing true false)
      (Variables|Default|SetTypeOfCrossroad 0))
    (:1
      (goto _label))
    (:2
      (Transformation|SetRelativeLocation _r_railing_2 (Math|Vector|MakeVector 0.0 -55.0 0.0) false false)
      (Rendering|SetVisibility _r_railing true false)
      (Variables|Default|SetTypeOfCrossroad 2)))
  (CallFunction|GetLaneTransforms)
  (|CallParentFunction))

(fn GetSpawnTransform
  (|CallParentFunction))

(fn SpawnNew
  (params (NewParam :type Actor%20Object%20Reference))
  (|CallParentFunction 0))

(fn SpawnObstacle)

(fn GetNextTransform
  (bind _nextspawnpoint_02 (Variables|Default|GetNextSpawnPoint_02))
  (bind _nextspawnpoint (Variables|Default|GetNextSpawnPoint))
  (bind _returnvalue (Transformation|GetWorldTransform _nextspawnpoint_02))
  (bind _returnvalue_2 (Transformation|GetWorldTransform _nextspawnpoint))
  (switch int (Variables|Default|GetTypeOfCrossroad)
    (:Default
      _)
    (:0
      _)
    (:1
      (return _returnvalue_2 _returnvalue))
    (:2
      (return _returnvalue "")))
  (return _returnvalue_2 ""))

(fn GetLaneTransforms
  (Variables|Default|SetRightLanes (Utilities|Array|MakeArray (Transformation|GetWorldTransform (Variables|Default|GetR_Lane_Left)) (Transformation|GetWorldTransform (Variables|Default|GetR_Lane_Mid)) (Transformation|GetWorldTransform (Variables|Default|GetR_Lane_Right))))
  (Variables|Default|SetLeftLanes (Utilities|Array|MakeArray (Transformation|GetWorldTransform (Variables|Default|GetL_Lane_Left)) (Transformation|GetWorldTransform (Variables|Default|GetL_Lane_Right)) (Transformation|GetWorldTransform (Variables|Default|GetL_Lane_Mid)))))