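; Collectible crystal coin pickup that spins constantly and awards its coin value when the player touches it.
; Overlap with the player starts a timeline that plays a chime once, pulls the actor toward the pawn's live position and shrinks it to zero.
; When the timeline finishes, it sends the points to RoadMaster through an interface message and destroys itself.
; A second timeline for moving the mesh between two points is left unconnected and never runs.
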(event OnComponentBeginOverlap(Sphere)
  (params (OverlappedComponent :type Primitive%20Component%20Object%20Reference) (OtherActor :type Actor%20Object%20Reference) (OtherComp :type Primitive%20Component%20Object%20Reference) (OtherBodyIndex :type Integer) (bFromSweep :type Boolean) (SweepResult :type Hit%20Result%20Structure%20%28by%20ref%29))
  (if (== OtherActor (Variables|Default|GetAs%20BP%20Player))
    (bind (_direction _move _size) (Timeline|Timeline_0 Play)
      (:Update
        (Utilities|FlowControl|Sequence
          (:then_0
            (Utilities|FlowControl|DoOnce false
              (:Completed
                (Audio|SpawnSound2D "/Game/TeachersMarketplace/Assets/SFX/SFX_Chime_03A.SFX_Chime_03A" 0.2 1.0 0.0 0))))
          (:then_1
            (Transformation|SetActorLocation (Math|Vector|Lerp(Vector) (Transformation|GetActorLocation) (Transformation|GetActorLocation (Game|Player|GetPlayerPawn 0)) _move) false false)
            (Transformation|SetActorScale3D (Math|Vector|Lerp(Vector) (Variables|Default|GetStart%20Scale) "0, 0, 0" _size)))))
      (:Finished
        (Class|BPIEndlessRoad|AddPointsInterface(Message) (Variables|Default|GetRoadMaster) (Variables|Default|GetCoinValue))
        (Actor|DestroyActor)))))

(event EventTick
  (params (DeltaSeconds :type Float%20%28single-precision%29))
  (Transformation|AddWorldRotation (Variables|Default|GetStaticMesh) "0,1.500000, 0" false false))

(event Collision|EventActorBeginOverlap
  (params (OtherActor :type Actor%20Object%20Reference)))

(event EventBeginPlay
  (|CallParentFunction) ; This node is disabled and will not be called.\nDrag off pins to build functionality.
)

(fn ConstructionScript
  (|CallParentFunction))