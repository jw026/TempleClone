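; BP_DestructableCube is an actor with a destructible mesh that fractures when something overlaps its box trigger.
; BeginPlay caches the player character and its left-hand collision component.
; Any box overlap, without checking the overlapping component, applies damage at the left hand's location with a fixed X-direction impulse.
; The hand-collision checks and other damage nodes are disconnected, and the hit events are empty.
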(event OnComponentBeginOverlap(Box)
  (params (OverlappedComponent :type Primitive%20Component%20Object%20Reference) (OtherActor :type Actor%20Object%20Reference) (OtherComp :type Primitive%20Component%20Object%20Reference) (OtherBodyIndex :type Integer) (bFromSweep :type Boolean) (SweepResult :type Hit%20Result%20Structure%20%28by%20ref%29))
  (Class|DestructibleComponent|ApplyDamage (Variables|Default|GetDestructible) 1e+01 (Transformation|GetWorldLocation (Variables|/Game/Blueprints/BP_Player.BP_Player_C|GetLeftHandCollision (Variables|Default|GetAs%20BP%20Player))) (Math|Vector|MakeVector 1e+02 0.0 0.0) 1e+02))

(event OnComponentHit(Destructible)
  (params (HitComponent :type Primitive%20Component%20Object%20Reference) (OtherActor :type Actor%20Object%20Reference) (OtherComp :type Primitive%20Component%20Object%20Reference) (NormalImpulse :type Vector :default "0, 0, 0") (Hit :type Hit%20Result%20Structure%20%28by%20ref%29)))

(event Custom|Destroy)

(event EventBeginPlay
  (bind _asbp_player (Utilities|Casting|CastToBP_Player (Game|GetPlayerCharacter 0)))
  (Variables|Default|SetAs%20BP%20Player _asbp_player)
  (Variables|Default|SetLeft%20Hand%20Collision (Variables|/Game/Blueprints/BP_Player.BP_Player_C|GetLeftHandCollision (Variables|Default|GetAs%20BP%20Player))))

(event Collision|EventHit
  (params (MyComp :type Primitive%20Component%20Object%20Reference) (Other :type Actor%20Object%20Reference) (OtherComp :type Primitive%20Component%20Object%20Reference) (bSelfMoved :type Boolean) (HitLocation :type Vector :default "0, 0, 0") (HitNormal :type Vector :default "0, 0, 0") (NormalImpulse :type Vector :default "0, 0, 0") (Hit :type Hit%20Result%20Structure%20%28by%20ref%29)))

(fn ConstructionScript)